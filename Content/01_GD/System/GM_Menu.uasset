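; Game mode for the local multiplayer menu and end-game levels.
; On BeginPlay it loads or creates the save, creates up to four local players with Enhanced Input, and refreshes the GI_PG level list.
; Player lobby states determine when starting is allowed; launching stores the player count and opens the first level after a transition.
; On end-game maps it spawns the top scorer and losers, then switches camera and shows the restart UI.
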(event `CheckSave`
  ;[1 0.3582 0.9385 1 25] Check Save
  (bind _returnvalue (`GameplayStatics.DoesSaveGameExist` "save1"))
  (if _returnvalue
    (bind _returnvalue_2 (`GameplayStatics.LoadGameFromSlot` "save1"))
    (bind _asbp_save_game (cast `/Game/01_GD/System/BP_SaveGame` _returnvalue_2))
    (set `self.SaveGame` _asbp_save_game)
    (else
      (bind _returnvalue_3 (`GameplayStatics.CreateSaveGameObject` "/Game/01_GD/System/BP_SaveGame.BP_SaveGame_C"))
      (`GameplayStatics.SaveGameToSlot` _returnvalue_3 "save1")
      (set `self.SaveGame` _returnvalue_3))))

(event `self.ReceiveBeginPlay`
  (bind _returnvalue (`GameplayStatics.GetPlayerController` 0))
  (bind _returnvalue_2 (`GameplayStatics.GetPlayerController` (`self.Array_Index`)))
  (`self.CheckSave`)
  (bind _asgi_pg (cast `/Game/01_GD/System/GI_PG` (`GameplayStatics.GetGameInstance`)))
  (set `self.GI_PG` _asgi_pg)
  (`|ExecutionSequence`
    (:`then_0`
      _)
    (:`then_1`
      (`self.EndGameMap?`)
      (`/Game/01_GD/System/GI_PG.SetGlobalLevelList` (`self.GI_PG`))))
  ;[1 0.246 0.1962 1 50] Multiplayer Gestion
  (for _index (range 4)
    (set `self.Array_Index` _index)
    (bind _returnvalue_3 (`GameplayStatics.CreatePlayer` (`self.Array_Index`)))
    (set `self.ControllerRef` _returnvalue_3)
    (if (> (`self.Array_Index`) 0)
      (`/Engine/EditorBlueprintResources/StandardMacros.IsValid` (`self.ControllerRef`)
        (:`Is Valid`
          (`EnhancedInputSubsystemInterface.AddMappingContext` (pcsubsystem `EnhancedInputLocalPlayerSubsystem` (`self.ControllerRef`)) "/Game/01_GD/Inputs/IMC_Player.IMC_Player" 0 (struct))
          (bind _aspc_menu (cast `/Game/01_GD/System/PC_Menu` (`self.ControllerRef`)))
          (set `/Game/01_GD/System/PC_Menu.ID` (`self.Array_Index`) _aspc_menu))
        (:`Is Not Valid`
          ;;[1 0.6776 0.3656 1 25] If the PC was created before (he is in cache)
          (`EnhancedInputSubsystemInterface.AddMappingContext` (pcsubsystem `EnhancedInputLocalPlayerSubsystem` _returnvalue_2) "/Game/01_GD/Inputs/IMC_Player.IMC_Player" 0 (struct))
          (bind _aspc_menu_2 (cast `/Game/01_GD/System/PC_Menu` _returnvalue_2))
          (set `/Game/01_GD/System/PC_Menu.ID` (`self.Array_Index`) _aspc_menu_2)))
      (else
        ;;[1 0.6776 0.3656 1 25] If we are P1
        (`EnhancedInputSubsystemInterface.AddMappingContext` (pcsubsystem `EnhancedInputLocalPlayerSubsystem` _returnvalue) "/Game/01_GD/Inputs/IMC_Player.IMC_Player" 0 (struct))
        (`WidgetBlueprintLibrary.SetInputMode_GameOnly` _returnvalue)))))

(event `CheckStates`
  ;[1 0.7299 0.2581 1 50] Check States to start game
  (set `self.PlayerReady` 0)
  (set `self.PlayerNotReady` 0)
  (for _array_element (`self.PlayerShows`)
    (bind _state (`/Game/01_GD/Gameplay/3DText/PlayerShow.State` _array_element))
    (if (== _state 2)
      (`/Engine/EditorBlueprintResources/StandardMacros.IncrementInt` (`self.PlayerReady`))
      (elif (== _state 1)
        (`/Engine/EditorBlueprintResources/StandardMacros.IncrementInt` (`self.PlayerNotReady`)))))
  (if (and (== (`self.PlayerNotReady`) 0) (> (`self.PlayerReady`) 1))
    (`KismetSystemLibrary.PrintString` "READY" true true (struct :`R` 1.0 :`B` 0.944322 :`A` 1.0) 5.0)
    (`self.SetActorHiddenInGame` (`self.StartGameWidget`) false)
    (set `self.CanStart?` true)
    (else
      (`KismetSystemLibrary.PrintString` "NOT READY" true true (struct :`R` 1.0 :`B` 0.944322 :`A` 1.0) 5.0)
      (`self.SetActorHiddenInGame` (`self.StartGameWidget`) true)
      (set `self.CanStart?` false))))

(event `LaunchGame`
  ;[0.3176 0.6444 1 1 25] LaunchGame
  (`/Engine/EditorBlueprintResources/StandardMacros.DoOnce` false
    (:`Completed`
      (`self.CheckStates`)
      (bind _asgi_pg (cast `/Game/01_GD/System/GI_PG` (`GameplayStatics.GetGameInstance`)))
      (set `/Game/01_GD/System/GI_PG.HowManyPlayers` (`self.PlayerReady`) _asgi_pg)
      (`GameplayStatics.PlaySound2D` "/Game/05_SD/Cues/Sounds/StartSound_Cue.StartSound_Cue" 1.0 1.0 0.0 null null)
      (bind _returnvalue (`|CreateWidget` "/Game/01_GD/UI/UI_EndTransition.UI_EndTransition_C" (`GameplayStatics.GetPlayerController` 0)))
      (`UserWidget.AddToViewport` _returnvalue 0)
      (`KismetSystemLibrary.Delay` 1.0)
      (`/Game/01_GD/System/GI_PG.OpenFirstLevel` (`self.GI_PG`)))))

(event `EndGameMap?`
  (bind _output (`|GetArrayItem` (`self.Materials`) (`KismetMathLibrary.MaxOfIntArray` (`/Game/01_GD/System/GI_PG.PlayersScore` (`self.GI_PG`)))))
  ;[1 0.2188 0.2188 1 50] END Maps
  (bind _returnvalue (`GameplayStatics.GetCurrentLevelName` true))
  (if (`KismetStringLibrary.Contains` _returnvalue "Level_EndGame")
    (set `self.Menu` "END")
    (`/Game/01_GD/System/GI_PG.PlayComment` (`self.GI_PG`) "NewEnumerator5")
    (bind _returnvalue_2 (`|CreateWidget` "/Game/01_GD/UI/UI_StartLevel.UI_StartLevel_C" (`GameplayStatics.GetPlayerController` 0)))
    (`UserWidget.AddToViewport` _returnvalue_2 0)
    ;;[0.7126 1 0.7915 1 25] Winner
    (bind _returnvalue_3 (`GameplayStatics.GetActorOfClass` "/Script/Engine.PlayerStart"))
    (`|SpawnActorFromClass` "/Game/01_GD/AI/AI_Winner.AI_Winner_C" (`self.GetTransform` _returnvalue_3) "Undefined" "MultiplyWithRoot" null _output null)
    (`KismetArrayLibrary.Array_RemoveItem` (`self.Materials`) _output)
    (bind _outactors (`GameplayStatics.GetAllActorsOfClass` "/Script/Engine.TargetPoint"))
    ;;[1 0.5932 0.5832 1 25] Loosers
    (set `self.TargetPoints` _outactors)
    (for (_array_element _array_index) (`self.Materials`)
      (if (< (+ _array_index 1) (`/Game/01_GD/System/GI_PG.HowManyPlayers` (`self.GI_PG`)))
        (`|SpawnActorFromClass` "/Game/01_GD/AI/AI_Looser.AI_Looser_C" (`self.GetTransform` (`|GetArrayItem` (`self.TargetPoints`) _array_index)) "Undefined" "MultiplyWithRoot" null _array_element null) ; Je spawn le dernier joueur possible à la place
      ))
    ;;[0.5578 0.8893 1 1 25] Switching Cam
    (`KismetSystemLibrary.Delay` 4.0)
    (bind _outactors_2 (`GameplayStatics.GetAllActorsOfClass` "/Game/01_GD/System/BP_Menu_Cam.BP_Menu_Cam_C"))
    (for _array_element_2 _outactors_2
      (if (== (`/Game/01_GD/System/BP_Menu_Cam.ID` _array_element_2) 1)
        (`/Game/01_GD/System/BP_Menu_Cam.SwitchCam` _array_element_2)
        (bind _returnvalue_4 (`|CreateWidget` "/Game/01_GD/UI/UI_Restart.UI_Restart_C" (`GameplayStatics.GetPlayerController` 0)))
        (set `self.UI_Restart` _returnvalue_4)
        (`UserWidget.AddToViewport` _returnvalue_4 0)))
    (else
      (`/Game/01_GD/System/GI_PG.PlayComment` (`self.GI_PG`) "NewEnumerator0"))))

(fn `ENDGAMEMusic`
  (bind _returnvalue (`GameplayStatics.GetCurrentLevelName` true))
  (bind _returnvalue_2 (`|GetDataTableRow` "/Game/01_GD/System/DT_Level.DT_Level" (`KismetStringLibrary.Conv_StringToName` _returnvalue))
    (:`then`
      (if (`KismetStringLibrary.EqualEqual_StrStr` (`.Mode_20_A2F9F94A43A2E094C1CC58AE455E7EC5` (break `/Game/01_GD/System/S_Level` _returnvalue_2)) "END")
        (`GameplayStatics.PlaySound2D` "/Game/05_SD/Cues/Musics/Maps/MapEND_Cue.MapEND_Cue" 1.0 1.0 0.0 null null)))))

(fn `SpawnParticleReader`)

(fn `UserConstructionScript`)