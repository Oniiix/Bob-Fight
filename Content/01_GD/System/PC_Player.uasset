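; PC_Player is the player controller for the party game, handling each player's map vote input.
; On BeginPlay it caches GM_PartyGame and, after a short delay, copies its ID onto the possessed BP_PG_Player pawn.
; The Attack, Y and Dash Enhanced Input actions each send one of three vote choices with that ID to the game mode's UIListMap, only while that widget is valid.
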(event `self.ReceiveBeginPlay`
  (bind _asgm_party_game (cast `/Game/01_GD/System/GM_PartyGame` (`GameplayStatics.GetGameMode`)))
  (set `self.GM` _asgm_party_game)
  (`KismetSystemLibrary.Delay` 0.1)
  (bind _asbp_pg_player (cast `/Game/01_GD/Player/BP_PG_Player` (`self.K2_GetPawn`)))
  (set `/Game/01_GD/Player/BP_PG_Player.ID` (`self.ID`) _asbp_pg_player))

(event `EnhancedInput|/Game/01_GD/Inputs/InputActions/IA_Attack`
  (params (ActionValue :type Boolean) (ElapsedSeconds :type "Float (double-precision)") (TriggeredSeconds :type "Float (double-precision)") (InputAction :type "InputAction Object Reference" :default "/Game/01_GD/Inputs/InputActions/IA_Attack.IA_Attack"))
  (bind _ui_listmap (`/Game/01_GD/System/GM_PartyGame.UI_ListMap` (`self.GM`)))
  (:`Started`
    (`/Engine/EditorBlueprintResources/StandardMacros.IsValid` _ui_listmap
      (:`Is Valid`
        (`/Game/01_GD/UI/UI_ListMaps.AddVoteF` _ui_listmap 0 (`self.ID`))))))

(event `EnhancedInput|/Game/01_GD/Inputs/InputActions/IA_Y`
  (params (ActionValue :type Boolean) (ElapsedSeconds :type "Float (double-precision)") (TriggeredSeconds :type "Float (double-precision)") (InputAction :type "InputAction Object Reference" :default "/Game/01_GD/Inputs/InputActions/IA_Y.IA_Y"))
  (bind _ui_listmap (`/Game/01_GD/System/GM_PartyGame.UI_ListMap` (`self.GM`)))
  (:`Started`
    (`/Engine/EditorBlueprintResources/StandardMacros.IsValid` _ui_listmap
      (:`Is Valid`
        (`/Game/01_GD/UI/UI_ListMaps.AddVoteF` _ui_listmap 1 (`self.ID`))))))

(event `EnhancedInput|/Game/01_GD/Inputs/InputActions/IA_Dash`
  (params (ActionValue :type Boolean) (ElapsedSeconds :type "Float (double-precision)") (TriggeredSeconds :type "Float (double-precision)") (InputAction :type "InputAction Object Reference" :default "/Game/01_GD/Inputs/InputActions/IA_Dash.IA_Dash"))
  (bind _ui_listmap (`/Game/01_GD/System/GM_PartyGame.UI_ListMap` (`self.GM`)))
  (:`Started`
    (`/Engine/EditorBlueprintResources/StandardMacros.IsValid` _ui_listmap
      (:`Is Valid`
        (`/Game/01_GD/UI/UI_ListMaps.AddVoteF` _ui_listmap 2 (`self.ID`))))))

(fn `UserConstructionScript`)