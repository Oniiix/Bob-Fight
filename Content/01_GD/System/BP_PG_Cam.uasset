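; BP_PG_Cam is the shared party-game camera that frames all BP_PG_Player actors in one view.
; On BeginPlay, after short delays for spawning, it becomes player 0's view target, gathers the players and registers with GM_PartyGame.
; Each tick it moves to the players' average location and spring-interpolates the SpringArm length from their largest separation, within clamped limits.
; SetCamera reapplies it as the view target.
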(event `self.ReceiveBeginPlay`
  ;[0.5289 0.5689 1 1 50] Get Players Refs
  (`KismetSystemLibrary.Delay` 0.001) ; They need to spawn, Don't move me
  (`PlayerController.SetViewTargetWithBlend` (`GameplayStatics.GetPlayerController` 0) self 0.0 "VTBlend_Linear" 0.0 false)
  (`KismetSystemLibrary.Delay` 0.001) ; They need to spawn
  (`KismetArrayLibrary.Array_Clear` (`self.Players`))
  (bind _outactors (`GameplayStatics.GetAllActorsOfClass` "/Game/01_GD/Player/BP_PG_Player.BP_PG_Player_C"))
  (for _array_element _outactors
    (`KismetArrayLibrary.Array_AddUnique` (`self.Players`) _array_element))
  (bind _asgm_party_game (cast `/Game/01_GD/System/GM_PartyGame` (`GameplayStatics.GetGameMode`))) ; Ref
  (set `/Game/01_GD/System/GM_PartyGame.Camera` self _asgm_party_game))

(event `SetCamera`
  ;[1 0 0.03471 1 25] To keep this camera active
  (`PlayerController.SetViewTargetWithBlend` (`GameplayStatics.GetPlayerController` 0) self 0.0 "VTBlend_Linear" 0.0 false))

(event `self.ReceiveTick`
  (params (DeltaSeconds :type "Float (single-precision)"))
  (bind _playersloc (`self.PlayersLoc`))
  (bind _springarm (`self.SpringArm`))
  (bind (_result_x _result_y _result_z) (`KismetMathLibrary.BreakVector` (`self.Result`)))
  (bind _playersloc_2 (`self.PlayersLoc`))
  ;[0.2964 0.7018 1 1 50] Camera Location
  (set `self.DeltaSeconds` DeltaSeconds)
  (`KismetArrayLibrary.Array_Clear` (`self.PlayersLoc`))
  (`KismetArrayLibrary.Array_Clear` (`self.DistancesBtwPlayers`))
  (set `self.Addition` (0.0 0.0 0.0))
  (for (_array_element _array_index) (`self.Players`)
    (`KismetArrayLibrary.Array_Set` (`self.PlayersLoc`) _array_index (`self.K2_GetActorLocation` _array_element) true))
  (for _array_element_2 _playersloc_2
    (set `self.Addition` (+ (`self.Addition`) _array_element_2)))
  (set `self.Result` (/ (`self.Addition`) (`KismetArrayLibrary.Array_Length` _playersloc_2)))
  (`self.K2_SetActorLocation` (`KismetMathLibrary.MakeVector` _result_x _result_y _result_z))
  ;[0.4316 1 0.7528 1 50] Camera Zoom
  (for (_array_element_3 _array_index_2) _playersloc
    (for _index (range (+ (`KismetArrayLibrary.Array_LastIndex` _playersloc) 1))
      (bind _returnvalue (`KismetMathLibrary.Vector_Distance` _array_element_3 (`|GetArrayItem` _playersloc _index)))
      (if (> _returnvalue (`|GetArrayItem` (`self.DistancesBtwPlayers`) _array_index_2))
        (`KismetArrayLibrary.Array_Set` (`self.DistancesBtwPlayers`) _array_index_2 _returnvalue true)))
    (bind _returnvalue_2 (`KismetMathLibrary.FloatSpringInterp` (`SpringArmComponent.TargetArmLength` _springarm) (`KismetMathLibrary.FClamp` (/ (* (`.MaxValue` (`KismetMathLibrary.MaxOfFloatArray` (`self.DistancesBtwPlayers`))) 2000.0) 1500.0) 500.0 1200.0) (`self.SpringState`) 10.0 1.0 (`self.DeltaSeconds`)))
    (set `SpringArmComponent.TargetArmLength` _returnvalue_2 _springarm)))

(fn `UserConstructionScript`)