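; Game mode for a local multiplayer party game that loads or creates the save, spawns players at shuffled starts and runs each round.
; The level's DT_Level row picks the music and hazard logic: bombs, rising lava tiles, zombies or fireballs.
; Deathmatch spawns recursively, giving players outside its roster spare pawns.
; PlayerDied records elimination order, hands dead players spare pawns, and shows scores when one survivor remains.
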(event `CheckSave`
  ;[1 0.3582 0.9385 1 25] Check Save
  (bind _returnvalue (`GameplayStatics.DoesSaveGameExist` "save1"))
  (if _returnvalue
    (bind _returnvalue_2 (`GameplayStatics.LoadGameFromSlot` "save1"))
    (bind _asbp_save_game (cast `/Game/01_GD/System/BP_SaveGame` _returnvalue_2))
    (set `self.SaveGame` _asbp_save_game)
    (else
      (bind _returnvalue_3 (`GameplayStatics.CreateSaveGameObject` "/Game/01_GD/System/BP_SaveGame.BP_SaveGame_C"))
      (`GameplayStatics.SaveGameToSlot` _returnvalue_3 "save1")
      (set `self.SaveGame` _returnvalue_3))))

(event `DeathmatchMulti`
  (bind _controllerref (`self.ControllerRef`))
  (bind _deathmatchindex (`self.DeathmatchIndex`))
  (bind _deathmatchindex_2 (`self.DeathmatchIndex`))
  (bind _returnvalue (`GameplayStatics.GetPlayerController` (`self.DeathmatchIndex`)))
  (bind _output (`|GetArrayItem` (`self.Playerstarts`) _deathmatchindex_2))
  (bind _returnvalue_2 (== (`KismetArrayLibrary.Array_Find` (`/Game/01_GD/System/GI_PG.DeathMatchPlayersIndex` (`self.GI_PG`)) _deathmatchindex) -1))
  ;[1 0.1546 0.2044 1 25] DeathMatch Multiplayer
  (`/Engine/EditorBlueprintResources/StandardMacros.IsValid` _output
    (:`Is Valid`
      (set `self.SpawnTransform` (`self.GetTransform` _output)))
    (:`Is Not Valid`
      _))
  (if (not (> _deathmatchindex_2 (- (`/Game/01_GD/System/GI_PG.HowManyPlayers` (`self.GI_PG`)) 1)))
    (bind _returnvalue_3 (`GameplayStatics.CreatePlayer` (`self.DeathmatchIndex`)))
    (set `self.ControllerRef` _returnvalue_3)
    (if (> (`self.DeathmatchIndex`) 0)
      (`/Engine/EditorBlueprintResources/StandardMacros.IsValid` (`self.ControllerRef`)
        (:`Is Valid`
          (`EnhancedInputSubsystemInterface.AddMappingContext` (pcsubsystem `EnhancedInputLocalPlayerSubsystem` (`self.ControllerRef`)) "/Game/01_GD/Inputs/IMC_Player.IMC_Player" 0 (struct))
          (if _returnvalue_2
            (`self.TakeTargetControl_DM` _deathmatchindex :!label _label)
            (`KismetArrayLibrary.Array_Add` (`self.Order`)) ; AddanEmptyPlace
            (else
              (bind _returnvalue_4 (`|SpawnActorFromClass` "/Game/01_GD/Player/BP_PG_Player.BP_PG_Player_C" (`self.SpawnTransform`) "Undefined" "MultiplyWithRoot" null null))
              (`Controller.Possess` _controllerref _returnvalue_4)
              (bind _aspc_player (cast `/Game/01_GD/System/PC_Player` _controllerref))
              (set `/Game/01_GD/System/PC_Player.ID` (`self.DeathmatchIndex`) _aspc_player))))
        (:`Is Not Valid`
          (`EnhancedInputSubsystemInterface.AddMappingContext` (pcsubsystem `EnhancedInputLocalPlayerSubsystem` _returnvalue) "/Game/01_GD/Inputs/IMC_Player.IMC_Player" 0 (struct))
          (if _returnvalue_2
            (goto _label)
            (else
              (bind _returnvalue_5 (`|SpawnActorFromClass` "/Game/01_GD/Player/BP_PG_Player.BP_PG_Player_C" (`self.SpawnTransform`) "Undefined" "MultiplyWithRoot" null null))
              (`Controller.Possess` _returnvalue _returnvalue_5)
              (bind _aspc_player_2 (cast `/Game/01_GD/System/PC_Player` _returnvalue))
              (set `/Game/01_GD/System/PC_Player.ID` (`self.DeathmatchIndex`) _aspc_player_2)))))
      (else
        ;;[1 0.6776 0.3656 1 25] If we are P1
        (`EnhancedInputSubsystemInterface.AddMappingContext` (pcsubsystem `EnhancedInputLocalPlayerSubsystem` (`GameplayStatics.GetPlayerController` 0)) "/Game/01_GD/Inputs/IMC_Player.IMC_Player" 0 (struct))
        (if (== (`KismetArrayLibrary.Array_Find` (`/Game/01_GD/System/GI_PG.DeathMatchPlayersIndex` (`self.GI_PG`)) (`self.DeathmatchIndex`)) -1)
          (goto _label)
          (else
            (bind _returnvalue_6 (`|SpawnActorFromClass` "/Game/01_GD/Player/BP_PG_Player.BP_PG_Player_C" (`self.SpawnTransform`) "Undefined" "MultiplyWithRoot" null null))
            (`Controller.Possess` (`GameplayStatics.GetPlayerController` 0) _returnvalue_6)))))
    (`/Engine/EditorBlueprintResources/StandardMacros.IncrementInt` (`self.DeathmatchIndex`) :!label _label_2
      (:`  `
        (`self.DeathmatchMulti`)))
    (else
      (bind _outactors (`GameplayStatics.GetAllActorsOfClass` "/Game/01_GD/Player/BP_PG_Player.BP_PG_Player_C"))
      (set `self.Players` _outactors)
      (`KismetSystemLibrary.Delay` 0.2) ; Casse les couilles
      (`/Game/01_GD/System/BP_PG_Cam.SetCamera` (`self.Camera`)))))

(event `self.ReceiveBeginPlay`
  (bind _controllerref (`self.ControllerRef`))
  (bind _returnvalue (`GameplayStatics.GetPlayerController` (`self.Array Index`)))
  (`self.CheckSave`)
  (`self.LevelModeAndMusic`)
  (bind _returnvalue_2 (`|CreateWidget` "/Game/01_GD/UI/UI_Start.UI_Start_C" (`GameplayStatics.GetPlayerController` 0)))
  (`UserWidget.AddToViewport` _returnvalue_2 0)
  (`self.SpawnParticleReader`)
  (bind _asgi_pg (cast `/Game/01_GD/System/GI_PG` (`GameplayStatics.GetGameInstance`)))
  (set `self.GI_PG` _asgi_pg)
  (bind _outactors (`GameplayStatics.GetAllActorsOfClass` "/Script/Engine.PlayerStart"))
  (bind _output_get (set `self.Playerstarts` _outactors))
  (`KismetArrayLibrary.Array_Shuffle` _output_get)
  ;[1 0.246 0.1962 1 50] Multiplayer Gestion
  (bind _returnvalue_3 (`GameplayStatics.GetCurrentLevelName` true))
  (bind _returnvalue_4 (`|GetDataTableRow` "/Game/01_GD/System/DT_Level.DT_Level" (`KismetStringLibrary.Conv_StringToName` _returnvalue_3))
    (:`then`
      (if (`KismetStringLibrary.EqualEqual_StrStr` (`.Mode_20_A2F9F94A43A2E094C1CC58AE455E7EC5` (break `/Game/01_GD/System/S_Level` _returnvalue_4)) "DEATHMATCH")
        (`self.DeathmatchMulti`)
        (else
          (for (_array_element _array_index) (`self.Playerstarts`)
            (set `self.Array Index` _array_index)
            (set `self.SpawnTransform` (`self.GetTransform` _array_element))
            (if (not (> _array_index (- (`/Game/01_GD/System/GI_PG.HowManyPlayers` (`self.GI_PG`)) 1)))
              (bind _returnvalue_5 (`GameplayStatics.CreatePlayer` (`self.Array Index`)))
              (set `self.ControllerRef` _returnvalue_5)
              (if (> (`self.Array Index`) 0)
                (`/Engine/EditorBlueprintResources/StandardMacros.IsValid` (`self.ControllerRef`)
                  (:`Is Valid`
                    (`EnhancedInputSubsystemInterface.AddMappingContext` (pcsubsystem `EnhancedInputLocalPlayerSubsystem` (`self.ControllerRef`)) "/Game/01_GD/Inputs/IMC_Player.IMC_Player" 0 (struct))
                    (bind _returnvalue_6 (`|SpawnActorFromClass` "/Game/01_GD/Player/BP_PG_Player.BP_PG_Player_C" (`self.SpawnTransform`) "Undefined" "MultiplyWithRoot" null null))
                    (`Controller.Possess` _controllerref _returnvalue_6)
                    (bind _aspc_player (cast `/Game/01_GD/System/PC_Player` _controllerref))
                    (set `/Game/01_GD/System/PC_Player.ID` (`self.Array Index`) _aspc_player))
                  (:`Is Not Valid`
                    (`EnhancedInputSubsystemInterface.AddMappingContext` (pcsubsystem `EnhancedInputLocalPlayerSubsystem` _returnvalue) "/Game/01_GD/Inputs/IMC_Player.IMC_Player" 0 (struct))
                    (bind _returnvalue_7 (`|SpawnActorFromClass` "/Game/01_GD/Player/BP_PG_Player.BP_PG_Player_C" (`self.SpawnTransform`) "Undefined" "MultiplyWithRoot" null null))
                    (`Controller.Possess` _returnvalue _returnvalue_7)
                    (bind _aspc_player_2 (cast `/Game/01_GD/System/PC_Player` _returnvalue))
                    (set `/Game/01_GD/System/PC_Player.ID` (`self.Array Index`) _aspc_player_2)))
                (else
                  ;;[1 0.6776 0.3656 1 25] If we are P1
                  (`EnhancedInputSubsystemInterface.AddMappingContext` (pcsubsystem `EnhancedInputLocalPlayerSubsystem` (`GameplayStatics.GetPlayerController` 0)) "/Game/01_GD/Inputs/IMC_Player.IMC_Player" 0 (struct))
                  (bind _returnvalue_8 (`|SpawnActorFromClass` "/Game/01_GD/Player/BP_PG_Player.BP_PG_Player_C" (`self.SpawnTransform`) "Undefined" "MultiplyWithRoot" null null))
                  (`Controller.Possess` (`GameplayStatics.GetPlayerController` 0) _returnvalue_8)))
              (else
                (break))))
          (bind _outactors_2 (`GameplayStatics.GetAllActorsOfClass` "/Game/01_GD/Player/BP_PG_Player.BP_PG_Player_C"))
          (set `self.Players` _outactors_2))))))

(event `ENDRound`
  ;[0.2127 0.6603 1 1 50] END Round
  (`KismetSystemLibrary.Delay` 1.0)
  (`GameplayStatics.SetGamePaused` true)
  (`/Game/01_GD/UI/UI_SCORE.SetLastScores` (`self.UI_END`)))

(event `SpawnParticleReader`
  ;[0.396 1 0.6747 1 25] ParticleReader
  (bind _returnvalue (`|SpawnActorFromClass` "/Game/04_FX/FX/BP_ParticleReader.BP_ParticleReader_C" (`KismetMathLibrary.MakeTransform` (0.0 0.0 0.0)) "Undefined" "MultiplyWithRoot" null null))
  (set `self.ParticleReader` _returnvalue))

(event `TakeTargetControl_DM`
  (params (PlayerIndex :type Integer))
  (bind _output (`|GetArrayItem` (`self.DeadPlayerPawns`)))
  ;[0.7725 0.4455 1 1 25] Take Target Control
  (`KismetSystemLibrary.Delay` (* (`self.DeathmatchIndex`) 0.01))
  (`/Engine/EditorBlueprintResources/StandardMacros.IsValid` _output
    (:`Is Valid`
      (set `/Game/01_GD/Gameplay/PossessablePawns/M_PossessablePawn.ID` PlayerIndex _output)
      (`Controller.Possess` (`GameplayStatics.GetPlayerController` PlayerIndex) _output) ; Possess a GPE in a list
      (`self.K2_SetActorLocation` _output (0.0 0.0 0.0) false false)
      (`KismetArrayLibrary.Array_RemoveItem` (`self.DeadPlayerPawns`) _output)
      (goto _label_2))))

(event `FloorIsLava`
  ;[0.5953 0.5377 1 1 50] Floor Is Lava
  (bind _returnvalue (`GameplayStatics.GetActorOfClass` "/Game/01_GD/Gameplay/FIL/TileBase.TileBase_C"))
  (set `self.TileBase` _returnvalue)
  (bind _outactors (`GameplayStatics.GetAllActorsOfClass` "/Game/01_GD/Gameplay/PossessablePawns/BP_TargetPlayer.BP_TargetPlayer_C"))
  (set `self.TargetPlayers` _outactors)
  (`self.TileSpawning`))

(event `SpawnBullet`
  (bind _bulletspawned (`self.BulletSpawned`))
  (bind _bulletspawner (`self.BulletSpawner`))
  (bind _bulletspawner_2 (`self.BulletSpawner`))
  ;[0.4886 0.5173 1 1 50] Bullet Gestion
  (`KismetSystemLibrary.Delay` 3.0)
  (`/Game/01_GD/Gameplay/BP_BulletSpawner.SpawnBullet` (`|GetArrayItem` _bulletspawner (`KismetMathLibrary.RandomIntegerInRange` 0 (`KismetArrayLibrary.Array_LastIndex` _bulletspawner))))
  (`/Engine/EditorBlueprintResources/StandardMacros.IncrementInt` _bulletspawned
    (:`  `
      (if (>= _bulletspawned 3)
        (set `self.BulletSpawned` 0)
        (`/Game/01_GD/Gameplay/BP_BulletSpawner.SpawnBullet` (`|GetArrayItem` _bulletspawner_2 (`KismetMathLibrary.RandomIntegerInRange` 0 (`KismetArrayLibrary.Array_LastIndex` _bulletspawner_2))))))))

(event `BombGame`
  (bind _returnvalue (`KismetMathLibrary.RandomFloatInRange` -250.0 250.0))
  (bind _output (`|GetArrayItem` (`self.Players`) (`KismetMathLibrary.RandomIntegerInRange` 0 (- (`/Game/01_GD/System/GI_PG.HowManyPlayers` (`self.GI_PG`)) 1))))
  ;[0.5953 0.5377 1 1 50] Bomb
  (`KismetSystemLibrary.Delay` (`KismetMathLibrary.RandomFloatInRange` 1.0 2.5))
  (if (`/Game/01_GD/Player/BP_PG_Player.Dead?` _output) :!label _label_3
    (`KismetSystemLibrary.Delay` 0.01)
    (goto _label_3)
    (else
      (bind _output_get (set `self.PlayerBomb` _output))
      (`/Game/Macro_Library.For Loop With Delay and Break` 0.8 0 1
        (:`Loop`
          (bind _output_get_2 (set `self.PlayerBombSpawn_` (+ (`self.K2_GetActorLocation` _output_get) (`KismetMathLibrary.MakeVector` _returnvalue _returnvalue 1000.0))))
          (`|SpawnActorFromClass` "/Game/01_GD/Gameplay/BP_Bomb.BP_Bomb_C" (`KismetMathLibrary.MakeTransform` _output_get_2) "Undefined" "MultiplyWithRoot" null null))
        (:`Complete`
          (`self.BombGame`))))))

(event `TileSpawning`
  (bind (_waterloc_x _waterloc_y _waterloc_z) (`KismetMathLibrary.BreakVector` (`self.WaterLoc`)))
  ;[0.5953 0.5377 1 1 50] Floor Is Lava
  (`KismetSystemLibrary.Delay` (`self.FIL_SpawnDelay`))
  (`self.FiL_SpawnNewTile`)
  (`|ExecutionSequence`
    (:`then_0`
      (set `self.FIL_SpawnDelay` (`KismetMathLibrary.FClamp` (- (`self.FIL_SpawnDelay`) -0.1) 5.0 9.0))
      (`self.TileSpawning`)
      (`self.MoveTargetsUp`))
    (:`then_1`
      (`KismetSystemLibrary.Delay` 1.9)
      (`/Game/01_GD/Gameplay/FIL/TileBase.WaterAlert` (`self.TileBase`))
      (`KismetSystemLibrary.Delay` 2.0)
      (set `self.WaterLoc` (`self.K2_GetActorLocation` (`self.TileBase`)))
      (bind (_direction _newtrack_0) (`Timeline|FiLWaterT` :!via `PlayFromStart`)
        (:`Update`
          (`self.K2_SetActorLocation` (`self.TileBase`) (`KismetMathLibrary.MakeVector` _waterloc_x _waterloc_y (`KismetMathLibrary.Lerp` _waterloc_z (+ _waterloc_z 100.0) _newtrack_0)) false false))))))

(event `ZombieGame`
  ;[0.5953 0.5377 1 1 50] Zombie Game
  (`KismetSystemLibrary.K2_SetTimerDelegate` (delegate `Spawn`) 3.0 true))

(event `MoveTargetsUp`
  ;[0.5953 0.5377 1 1 50] Floor Is Lava
  (for _array_element (`self.TargetPlayers`)
    (`self.K2_SetActorLocation` _array_element (+ (`self.K2_GetActorLocation` _array_element) (0.0 0.0 100.0)) false false)))

(event `Spawn`
  (bind _zombiecount (`self.ZombieCount`))
  ;[0.5953 0.5377 1 1 50] Zombie Game
  (for _array_element (`self.ZombieSpawner`)
    (`/Game/01_GD/Gameplay/BP_ZombieSpawner.spawnZombie` _array_element)
    (`/Engine/EditorBlueprintResources/StandardMacros.IncrementInt` _zombiecount
      (:`  `
        (if (>= _zombiecount 30)
          (`/Engine/EditorBlueprintResources/StandardMacros.DoOnce` false
            (:`Completed`
              (bind _asparty_game_gi (cast `PartyGame_GI` (`GameplayStatics.GetGameInstance`)))
              (`PartyGame_GI.SetAchievement` _asparty_game_gi "ACH_Survivors"))))))))

(fn `FiL_SpawnNewTile`
  (locals (TileToSpawn_01 :type "Actor Class Reference") (TileToSpawn_02 :type "Actor Class Reference") (TileToSpawn_03 :type "Actor Class Reference"))
  (bind (_fil_spawn_location _fil_spawn_rotation) (`KismetMathLibrary.BreakTransform` (`self.FIL_Spawn`)))
  (bind (_fil_spawn_location_2 _fil_spawn_rotation_2) (`KismetMathLibrary.BreakTransform` (`self.FIL_Spawn`)))
  (bind (_fil_spawn_location_3 _fil_spawn_rotation_3) (`KismetMathLibrary.BreakTransform` (`self.FIL_Spawn`)))
  (bind _returnvalue (`self.GetTransform` (`self.TileBase`)))
  (set `self.FIL_Spawn` (`KismetMathLibrary.MakeTransform` (`KismetMathLibrary.MakeVector` (.x (.location _returnvalue)) (.y (.location _returnvalue)) (+ (.z (.location _returnvalue)) 2000.0)) (.rotation _returnvalue) (.scale _returnvalue)))
  (bind _returnvalue_2 (`GameplayStatics.GetCurrentLevelName` true))
  (if (`KismetStringLibrary.Contains` _returnvalue_2 "01")
    (set `local.TileToSpawn_01` (select `int` (`KismetMathLibrary.RandomIntegerInRange` 0 1) :`0` "/Game/01_GD/Gameplay/FIL/01_FIL/01_Tile_G1_01.01_Tile_G1_01_C" :`1` "/Game/01_GD/Gameplay/FIL/01_FIL/01_Tile_G1_02.01_Tile_G1_02_C" :!type "Actor Class Reference"))
    (set `local.TileToSpawn_02` (select `int` (`KismetMathLibrary.RandomIntegerInRange` 0 1) :`0` "/Game/01_GD/Gameplay/FIL/01_FIL/01_Tile_G2_01.01_Tile_G2_01_C" :`1` "/Game/01_GD/Gameplay/FIL/01_FIL/01_Tile_G2_02.01_Tile_G2_02_C" :!type "Actor Class Reference"))
    (set `local.TileToSpawn_03` (select `int` (`KismetMathLibrary.RandomIntegerInRange` 0 1) :`0` "/Game/01_GD/Gameplay/FIL/01_FIL/01_Tile_G3_01.01_Tile_G3_01_C" :`1` "/Game/01_GD/Gameplay/FIL/01_FIL/01_Tile_G3_02.01_Tile_G3_02_C" :!type "Actor Class Reference"))
    (else
      (set `local.TileToSpawn_01` (select `int` (`KismetMathLibrary.RandomIntegerInRange` 0 1) :`0` "/Game/01_GD/Gameplay/FIL/02_Tile_G1_01.02_Tile_G1_01_C" :`1` "/Game/01_GD/Gameplay/FIL/02_Tile_G1_02.02_Tile_G1_02_C" :!type "Actor Class Reference"))
      (set `local.TileToSpawn_02` (select `int` (`KismetMathLibrary.RandomIntegerInRange` 0 1) :`0` "/Game/01_GD/Gameplay/FIL/02_Tile_G2_01.02_Tile_G2_01_C" :`1` "/Game/01_GD/Gameplay/FIL/02_Tile_G2_02.02_Tile_G2_02_C" :!type "Actor Class Reference"))
      (set `local.TileToSpawn_03` (select `int` (`KismetMathLibrary.RandomIntegerInRange` 0 1) :`0` "/Game/01_GD/Gameplay/FIL/02_Tile_G3_01.02_Tile_G3_01_C" :`1` "/Game/01_GD/Gameplay/FIL/02_Tile_G3_02.02_Tile_G3_02_C" :!type "Actor Class Reference"))))
  (switch `int` (`self.FIL_Group`) ; Switching Group
    (:`Default`
      (set `self.FIL_Group` 1 :!label _label)
      (`|SpawnActorFromClass` (`local.TileToSpawn_03`) (`KismetMathLibrary.MakeTransform` _fil_spawn_location_3 _fil_spawn_rotation_3) "Undefined" "MultiplyWithRoot" null null))
    (:`1`
      (`/Engine/EditorBlueprintResources/StandardMacros.IncrementInt` (`self.FIL_Group`)
        (:`  `
          (`|SpawnActorFromClass` (`local.TileToSpawn_01`) (`KismetMathLibrary.MakeTransform` _fil_spawn_location _fil_spawn_rotation) "Undefined" "MultiplyWithRoot" null null))))
    (:`2`
      (`/Engine/EditorBlueprintResources/StandardMacros.IncrementInt` (`self.FIL_Group`)
        (:`  `
          (`|SpawnActorFromClass` (`local.TileToSpawn_02`) (`KismetMathLibrary.MakeTransform` _fil_spawn_location_2 _fil_spawn_rotation_2) "Undefined" "MultiplyWithRoot" null null))))
    (:`3`
      (goto _label)))
  (return))

(fn `LevelModeAndMusic`
  (bind _returnvalue (`GameplayStatics.GetCurrentLevelName` true))
  (bind _returnvalue_2 (`|GetDataTableRow` "/Game/01_GD/System/DT_Level.DT_Level" (`KismetStringLibrary.Conv_StringToName` _returnvalue))
    (:`then`
      (switch `string` (`.Mode_20_A2F9F94A43A2E094C1CC58AE455E7EC5` (break `/Game/01_GD/System/S_Level` _returnvalue_2)) ; Oui...
        (:`BOMB`
          (`self.BombGame`)
          (`GameplayStatics.PlaySound2D` "/Game/05_SD/Cues/Musics/Maps/MapBomb_Cue.MapBomb_Cue" 1.0 1.0 0.0 null null))
        (:`FLOOR IS LAVA`
          (`self.FloorIsLava`)
          (`GameplayStatics.PlaySound2D` "/Game/05_SD/Cues/Musics/Maps/MapFIL_Cue.MapFIL_Cue" 1.0 1.0 0.0 null null))
        (:`ZOMBIE`
          (`self.ZombieGame`)
          (`GameplayStatics.PlaySound2D` "/Game/05_SD/Cues/Musics/Maps/MapZombie_Cue.MapZombie_Cue" 1.0 1.0 0.0 null null))
        (:`FIREBALL`
          (`self.SpawnBullet`)
          (`GameplayStatics.PlaySound2D` "/Game/05_SD/Cues/Musics/Maps/MapMask_Cue.MapMask_Cue" 1.0 1.0 0.0 null null))
        (:`SHARK`
          (`GameplayStatics.PlaySound2D` "/Game/05_SD/Cues/Musics/Maps/MapMask_Cue.MapMask_Cue" 1.0 1.0 0.0 null null))
        (:`DEATHMATCH`
          (`GameplayStatics.PlaySound2D` "/Game/05_SD/Cues/Musics/Maps/MapDEATHMATCH_Cue.MapDEATHMATCH_Cue" 1.0 1.0 0.0 null null)))
      (`GameplayStatics.PlaySound2D` "/Game/05_SD/Cues/Sounds/Crowd_Cue.Crowd_Cue" 1.0 1.0 0.0 null null))))

(fn `PlayerDied`
  (params (PlayerWhoDied :type "/Game/01_GD/Player/BP_PG_Player Object Reference"))
  (bind _id (`/Game/01_GD/Player/BP_PG_Player.ID` PlayerWhoDied))
  (bind _order (`self.Order`))
  (bind _output (`|GetArrayItem` (`self.DeadPlayerPawns`)))
  (`PrimitiveComponent.SetRenderCustomDepth` (`Character.Mesh` PlayerWhoDied) false)
  (`PrimitiveComponent.SetCollisionEnabled` (`Character.CapsuleComponent` PlayerWhoDied) "NoCollision")
  (`KismetArrayLibrary.Array_AddUnique` _order PlayerWhoDied)
  (bind _returnvalue (`|CreateWidget` "/Game/01_GD/UI/UI_Public.UI_Public_C" (`GameplayStatics.GetPlayerController` 0)))
  (`UserWidget.AddToViewport` _returnvalue 0)
  (if (== (`KismetArrayLibrary.Array_Length` _order) (- (`/Game/01_GD/System/GI_PG.HowManyPlayers` (`self.GI_PG`)) 1))
    ;[1 0.3008 0.9598 1 25] END ROUND
    (for _array_element (`self.Players`)
      (if (== (`KismetArrayLibrary.Array_Find` (`self.Order`) _array_element) -1)
        (`KismetArrayLibrary.Array_AddUnique` (`self.Order`) _array_element)))
    (`KismetArrayLibrary.Array_Reverse` (`self.Order`))
    (bind _returnvalue_2 (`|CreateWidget` "/Game/01_GD/UI/UI_SCORE.UI_SCORE_C" (`GameplayStatics.GetPlayerController` 0)))
    (bind _output_get (set `self.UI_END` _returnvalue_2))
    (`UserWidget.AddToViewport` _output_get 0)
    (`self.ENDRound`)
    (`/Game/01_GD/System/GI_PG.PlayComment` (`self.GI_PG`) "NewEnumerator7")
    (return)
    (else
      ;[0.4678 0.9701 1 1 25] POSSESS
      (`/Engine/EditorBlueprintResources/StandardMacros.IsValid` _output
        (:`Is Valid`
          (set `/Game/01_GD/Gameplay/PossessablePawns/M_PossessablePawn.ID` _id _output)
          (`Controller.Possess` (`GameplayStatics.GetPlayerController` _id) _output) ; Possess a GPE in a list
          (`self.K2_SetActorLocation` _output (`/Game/01_GD/System/BP_PG_Cam.Result` (`self.Camera`)) false false)
          (`KismetArrayLibrary.Array_RemoveItem` (`self.DeadPlayerPawns`) _output)
          (`/Game/01_GD/System/BP_PG_Cam.SetCamera` (`self.Camera`))
          (`/Game/01_GD/System/GI_PG.PlayComment` (`self.GI_PG`) "NewEnumerator3")
          (return))))))

(fn `UserConstructionScript`)