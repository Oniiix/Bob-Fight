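; BP_Menu_Cam is a menu camera that can become the player's view target.
; On BeginPlay it registers itself in the CamMenu array of the GM_Menu game mode at the index given by its ID.
; The camera with ID 0 takes the view immediately as the starting shot.
; Its SwitchCam event blends the player's view to that camera over a short transition.
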(event `self.ReceiveBeginPlay`
  (bind _asgm_menu (cast `/Game/01_GD/System/GM_Menu` (`GameplayStatics.GetGameMode`)))
  (`KismetArrayLibrary.Array_Set` (`/Game/01_GD/System/GM_Menu.CamMenu` _asgm_menu) (`self.ID`) self true)
  (if (== (`self.ID`) 0)
    (`PlayerController.SetViewTargetWithBlend` (`GameplayStatics.GetPlayerController` 0) self 0.0 "VTBlend_Linear" 0.0 false)))

(event `SwitchCam`
  (`PlayerController.SetViewTargetWithBlend` (`GameplayStatics.GetPlayerController` 0) self 1.5 "VTBlend_Linear" 0.0 false))

(fn `UserConstructionScript`)