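; Timed bomb that explodes shortly after BeginPlay, knocking back nearby actors and breaking destroyables.
; After a delay, a Timeline animates a dynamic material's emissive as a fuse, then calls Explosion on finish.
; Explosion plays sound and Niagara VFX, then a wide sphere trace launches players and enemies and shoves other bombs away with added lift.
; A tighter trace destroys M_Destroyable actors before the bomb destroys itself.
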(event `self.ReceiveBeginPlay`
  (bind _dm (`self.DM`))
  (`KismetSystemLibrary.Delay` 2.0)
  (bind _returnvalue (`PrimitiveComponent.CreateDynamicMaterialInstance` (`self.PhysicalMesh`) 0 "/Game/Graph/Materials/MI_Bomb.MI_Bomb" "None"))
  (set `self.DM` _returnvalue)
  (bind (_direction _newtrack_0) (`Timeline|Timeline` :!via `PlayFromStart`)
    (:`Update`
      (`MaterialInstanceDynamic.SetVectorParameterValue` _dm "EmissiveMultiplier" _newtrack_0)
      (`MaterialInstanceDynamic.SetTextureParameterValue` _dm "BaseColor" "/Game/Graph/Japanese_Street/Textures/AE_House/AE_Floor_01/AE_Floor_A.AE_Floor_A"))
    (:`Finished`
      (`self.Explosion`))))

(event `Explosion`
  (bind _returnvalue (`SceneComponent.K2_GetComponentLocation` (`self.PhysicalMesh`)))
  (bind _returnvalue_2 (`SceneComponent.K2_GetComponentLocation` (`self.PhysicalMesh`)))
  (`GameplayStatics.PlaySound2D` "/Game/05_SD/Wav/Firework/Explosion_Cue.Explosion_Cue" 1.0 1.0 0.0 null null)
  (`NiagaraFunctionLibrary.SpawnSystemAtLocation` "/Game/04_FX/Explosions_W3Vol1/Niagara/NS_Explosive5.NS_Explosive5" (`SceneComponent.K2_GetComponentLocation` (`self.PhysicalMesh`)))
  (`KismetSystemLibrary.Delay` 0.1)
  (`|ExecutionSequence`
    (:`then_0`
      (bind (_outhits _returnvalue_3) (`KismetSystemLibrary.SphereTraceMultiForObjects` _returnvalue_2 _returnvalue_2 300.0 (`|MakeArray` "ObjectTypeQuery3" "ObjectTypeQuery4" :!type "EObjectTypeQuery Enum")))
      ;[1 1 1] Impulse
      (if _returnvalue_3
        (for _array_element _outhits
          (`|ExecutionSequence`
            (:`then_0`
              (bind (_bblockinghit _binitialoverlap _time _distance _location _impactpoint _normal _impactnormal _physmat _hitactor _hitcomponent) (`GameplayStatics.BreakHitResult` _array_element))
              (bind _asbp_pg_player (cast `/Game/01_GD/Player/BP_PG_Player` _hitactor))
              (bind _returnvalue_4 (+ (* (`KismetMathLibrary.GetDirectionUnitVector` (`SceneComponent.K2_GetComponentLocation` (`self.PhysicalMesh`)) (`self.K2_GetActorLocation` _hitactor)) 500.0) (0.0 0.0 300.0)))
              (`Character.LaunchCharacter` _asbp_pg_player _returnvalue_4 true true))
            (:`then_1`
              (bind _asai_enemy (cast `/Game/01_GD/AI/AI_Enemy` _hitactor))
              (`Character.LaunchCharacter` _asai_enemy _returnvalue_4 true true))
            (:`then_2`
              (bind _asbp_bomb (cast `/Game/01_GD/Gameplay/BP_Bomb` _hitactor))
              (`PrimitiveComponent.AddImpulse` (`/Game/01_GD/Gameplay/BP_Bomb.PhysicalMesh` _asbp_bomb) (+ (* (`KismetMathLibrary.GetDirectionUnitVector` (`SceneComponent.K2_GetComponentLocation` (`self.PhysicalMesh`)) (`SceneComponent.K2_GetComponentLocation` _hitcomponent)) 300.0) (0.0 0.0 300.0)) "None" true))))))
    (:`then_1`
      (bind (_outhits_2 _returnvalue_5) (`KismetSystemLibrary.SphereTraceMultiForObjects` _returnvalue _returnvalue 90.0 (`|MakeArray` "ObjectTypeQuery1" "ObjectTypeQuery2" :!type "EObjectTypeQuery Enum")))
      (if _returnvalue_5
        (for _array_element_2 _outhits_2
          (bind _asm_destroyable (cast `/Game/01_GD/Gameplay/Destroyable/M_Destroyable` (`.HitActor` (`GameplayStatics.BreakHitResult` _array_element_2))))
          (`self.K2_DestroyActor` _asm_destroyable)))
      (`self.K2_DestroyActor`))))

(fn `UserConstructionScript`)