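; BP_Bullet is a party-game projectile that flies forward along its local X axis and explodes lethally.
; It detonates after a lifetime delay or when its sphere overlaps anything other than a BP_PlayerBulletSpawner, guarded by DoOnce.
; The explosion sphere-traces physics bodies with debug drawing, kills BP_PG_Player hits with an impulse and spawns ice VFX.
; It then asks GM_PartyGame to spawn another bullet and destroys itself.
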(event `self.ReceiveBeginPlay`
  (`KismetSystemLibrary.Delay` 10.0)
  (`self.Explosion`))

(event `self.ReceiveTick`
  (params (DeltaSeconds :type "Float (single-precision)"))
  (`self.K2_AddActorLocalOffset` (`KismetMathLibrary.MakeVector` (* DeltaSeconds (`self.Speed`)))))

(event `self.Sphere.OnComponentBeginOverlap`
  (params (OverlappedComponent :type "PrimitiveComponent Object Reference") (OtherActor :type "Actor Object Reference") (OtherComp :type "PrimitiveComponent Object Reference") (OtherBodyIndex :type Integer) (bFromSweep :type Boolean) (SweepResult :type "HitResult Structure (by ref)"))
  (cast `/Game/01_GD/Gameplay/PossessablePawns/BP_PlayerBulletSpawner` OtherActor
    (:`CastFailed`
      (`self.Explosion`))))

(event `Explosion`
  (bind _returnvalue (`self.K2_GetActorLocation`))
  ;[1 0.07955 0.1592 1 25] Explosion
  (`/Engine/EditorBlueprintResources/StandardMacros.DoOnce` false
    (:`Completed`
      (bind _outhits (`KismetSystemLibrary.SphereTraceMultiForObjects` :`Start` _returnvalue :`End` _returnvalue :`Radius` 150.0 :`ObjectTypes` (`|MakeArray` "ObjectTypeQuery4" :!type "EObjectTypeQuery Enum") :`DrawDebugType` "ForDuration"))
      (for _array_element _outhits
        (bind _asbp_pg_player (cast `/Game/01_GD/Player/BP_PG_Player` (`.HitActor` (`GameplayStatics.BreakHitResult` _array_element))))
        (`/Game/01_GD/Player/BP_PG_Player.DEATH` _asbp_pg_player true (`self.K2_GetActorLocation`) 1000.0))
      (`NiagaraFunctionLibrary.SpawnSystemAtLocation` "/Game/Graph/FX/NS/NS_Ice_Explode.NS_Ice_Explode" (`self.K2_GetActorLocation`))
      (bind _asgm_party_game (cast `/Game/01_GD/System/GM_PartyGame` (`GameplayStatics.GetGameMode`)))
      (`/Game/01_GD/System/GM_PartyGame.SpawnBullet` _asgm_party_game)
      (`self.K2_DestroyActor`))))

(fn `UserConstructionScript`)