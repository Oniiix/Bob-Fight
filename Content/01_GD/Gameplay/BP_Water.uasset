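; BP_Water is a water hazard actor that kills the player on touch and moves vertically.
; Two seconds after BeginPlay, the Movement timeline lerps the actor between its cached start location and a point 100 units above it.
; The UpMovement event replays that timeline from the start.
; Box overlap casts the other actor to BP_PG_Player and calls DEATH on it.
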(event `self.ReceiveBeginPlay`
  (bind _loc_init (`self.Loc_Init`))
  (set `self.Loc_Init` (`self.K2_GetActorLocation`))
  (`KismetSystemLibrary.Delay` 2.0)
  (bind (_direction _newtrack_0) (`Timeline|Movement` :!via `PlayFromStart` :!label _label)
    (:`Update`
      (`self.K2_SetActorLocation` (`KismetMathLibrary.VLerp` _loc_init (+ _loc_init (0.0 0.0 100.0)) _newtrack_0)))))

(event `UpMovement`
  (goto _label :!via `PlayFromStart`))

(event `self.Box.OnComponentBeginOverlap`
  (params (OverlappedComponent :type "PrimitiveComponent Object Reference") (OtherActor :type "Actor Object Reference") (OtherComp :type "PrimitiveComponent Object Reference") (OtherBodyIndex :type Integer) (bFromSweep :type Boolean) (SweepResult :type "HitResult Structure (by ref)"))
  (bind _asbp_pg_player (cast `/Game/01_GD/Player/BP_PG_Player` OtherActor))
  (`/Game/01_GD/Player/BP_PG_Player.DEATH` _asbp_pg_player))

(fn `UserConstructionScript`)