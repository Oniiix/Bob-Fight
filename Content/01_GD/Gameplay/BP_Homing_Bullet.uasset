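; Homing projectile for the party game that flies straight after spawning, then chases the nearest living player at a steadily increasing speed.
; Tick recomputes distances to the cached player list, giving dead players a huge distance, then moves and rotates toward the closest.
; Player overlap or a lifetime delay triggers Explosion, which kills players within a sphere trace, has GM_PartyGame spawn another bullet, and destroys itself.
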(event `self.ReceiveBeginPlay`
  (`|ExecutionSequence`
    (:`then_0`
      (`KismetSystemLibrary.Delay` 0.2)
      (bind _outactors (`GameplayStatics.GetAllActorsOfClass` "/Game/01_GD/Player/BP_PG_Player.BP_PG_Player_C"))
      (set `self.Players` _outactors)
      (`KismetSystemLibrary.Delay` 2.0)
      (set `self.Activated` true))
    (:`then_1`
      (`KismetSystemLibrary.K2_SetTimerDelegate` (delegate `AddSpeed`) 2.0 true) ; Adding Speed Loop
      (`KismetSystemLibrary.Delay` 10.0)
      (`self.Explosion`))))

(event `self.Sphere.OnComponentBeginOverlap`
  (params (OverlappedComponent :type "PrimitiveComponent Object Reference") (OtherActor :type "Actor Object Reference") (OtherComp :type "PrimitiveComponent Object Reference") (OtherBodyIndex :type Integer) (bFromSweep :type Boolean) (SweepResult :type "HitResult Structure (by ref)"))
  (cast `/Game/01_GD/Player/BP_PG_Player` OtherActor)
  (`self.Explosion`))

(event `AddSpeed`
  (set `self.Speed` (+ (`self.Speed`) 0.5)))

(event `self.ReceiveTick`
  (params (DeltaSeconds :type "Float (single-precision)"))
  (bind _returnvalue (`self.K2_GetActorLocation`))
  (bind _distancewithplayers (`self.DistanceWithPlayers`))
  (bind _returnvalue_2 (`self.K2_GetActorLocation` (`|GetArrayItem` (`self.Players`) (`KismetMathLibrary.MinOfFloatArray` (`self.DistanceWithPlayers`)))))
  ;[0.5354 1 0.8478 1 25] Homing Bullet
  (if (`self.Activated`)
    (`KismetArrayLibrary.Array_Clear` (`self.DistanceWithPlayers`))
    (for (_array_element _array_index) (`self.Players`)
      (if (`/Game/01_GD/Player/BP_PG_Player.Dead?` _array_element)
        (`KismetArrayLibrary.Array_Set` _distancewithplayers _array_index 100000.0 true) ; It will never be the nearest
        (else
          (`KismetArrayLibrary.Array_Set` _distancewithplayers _array_index (`self.GetDistanceTo` _array_element) true))))
    (`self.K2_AddActorWorldOffset` (* (`KismetMathLibrary.GetDirectionUnitVector` _returnvalue _returnvalue_2) (`self.Speed`)))
    (`self.K2_SetActorRotation` (`KismetMathLibrary.FindLookAtRotation` _returnvalue _returnvalue_2))
    (else
      (`self.K2_AddActorLocalOffset` (`KismetMathLibrary.MakeVector` (`self.Speed`))))))

(event `Explosion`
  (bind _returnvalue (`self.K2_GetActorLocation`))
  ;[1 0.125 0.4373 1 25] Explosion
  (`NiagaraFunctionLibrary.SpawnSystemAtLocation` "/Game/04_FX/FX/VFX_Explosion.VFX_Explosion" (`self.K2_GetActorLocation`))
  (`/Engine/EditorBlueprintResources/StandardMacros.DoOnce` false
    (:`Completed`
      (bind _outhits (`KismetSystemLibrary.SphereTraceMultiForObjects` _returnvalue _returnvalue 150.0 (`|MakeArray` "ObjectTypeQuery4" :!type "EObjectTypeQuery Enum")))
      (for _array_element _outhits
        (bind _asbp_pg_player (cast `/Game/01_GD/Player/BP_PG_Player` (`.HitActor` (`GameplayStatics.BreakHitResult` _array_element))))
        (`/Game/01_GD/Player/BP_PG_Player.DEATH` _asbp_pg_player true (`self.K2_GetActorLocation`) 600.0))
      (bind _asgm_party_game (cast `/Game/01_GD/System/GM_PartyGame` (`GameplayStatics.GetGameMode`)))
      (`/Game/01_GD/System/GM_PartyGame.SpawnBullet` _asgm_party_game)
      (`self.K2_DestroyActor`))))

(fn `UserConstructionScript`)