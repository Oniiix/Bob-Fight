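; BP_BulletSpawner is a spawn point that launches homing bullets in the party game.
; On BeginPlay it registers itself in the BulletSpawner array on GM_PartyGame.
; SpawnBullet plays a wind-explosion Niagara effect and spawns a BP_Homing_Bullet at the Scene component's transform, passing itself as the bullet's SpawnerOwner.
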(event `self.ReceiveBeginPlay`
  (bind _asgm_party_game (cast `/Game/01_GD/System/GM_PartyGame` (`GameplayStatics.GetGameMode`)))
  (`KismetArrayLibrary.Array_AddUnique` (`/Game/01_GD/System/GM_PartyGame.BulletSpawner` _asgm_party_game) self))

(event `SpawnBullet`
  (bind _returnvalue (`SceneComponent.K2_GetComponentToWorld` (`self.Scene`)))
  (`NiagaraFunctionLibrary.SpawnSystemAtLocation` "/Game/Graph/FX/NS/NS_Wind_explode.NS_Wind_explode" (.location _returnvalue) (.rotation _returnvalue) (.scale _returnvalue))
  (`|SpawnActorFromClass` "/Game/01_GD/Gameplay/BP_Homing_Bullet.BP_Homing_Bullet_C" _returnvalue "Undefined" "MultiplyWithRoot" null self null))

(fn `UserConstructionScript`)