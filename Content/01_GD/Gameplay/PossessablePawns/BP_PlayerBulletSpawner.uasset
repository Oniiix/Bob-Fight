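; BP_PlayerBulletSpawner is a player-controlled shooter that fires a bullet when the attack input starts.
; The IA_Attack Enhanced Input event calls SpawnBullet, which plays a Niagara wind-explosion effect and spawns a BP_Bullet at the Scene component's transform, owned by the spawner.
; An unconnected timeline that would swing RotScene's yaw from side to side never runs.
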(event `SpawnBullet`
  (bind _returnvalue (`SceneComponent.K2_GetComponentToWorld` (`self.Scene`)))
  ;[0.8987 0.1643 1 1 25] SpawnBullet
  (`NiagaraFunctionLibrary.SpawnSystemAtLocation` "/Game/Graph/FX/NS/NS_Wind_explode.NS_Wind_explode" (.location _returnvalue) (.rotation _returnvalue))
  (`|SpawnActorFromClass` "/Game/01_GD/Gameplay/BP_Bullet.BP_Bullet_C" (`KismetMathLibrary.MakeTransform` (.location _returnvalue) (.rotation _returnvalue)) "Undefined" "MultiplyWithRoot" null self null))

(event `EnhancedInput|/Game/01_GD/Inputs/InputActions/IA_Attack`
  (params (ActionValue :type Boolean) (ElapsedSeconds :type "Float (double-precision)") (TriggeredSeconds :type "Float (double-precision)") (InputAction :type "InputAction Object Reference" :default "/Game/01_GD/Inputs/InputActions/IA_Attack.IA_Attack"))
  ;[1 0.4969 0.2011 1 25] Attack
  (:`Started`
    (`KismetSystemLibrary.PrintString` "Attack" true true (struct :`G` 1.0 :`B` 0.096388 :`A` 1.0) 5.0)
    (`self.SpawnBullet`)))

(fn `UserConstructionScript`)