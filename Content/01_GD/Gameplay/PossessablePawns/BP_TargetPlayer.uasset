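; BP_TargetPlayer is a possessable target pawn that the player slides around with Enhanced Input to drop bombs.
; IA_Move applies local offsets scaled by Speed, and IA_Attack spawns BP_Bomb at SpawnPoint behind a short cooldown.
; Possession reveals the Decal and Drop components.
; An idle rumble using a looping Shake timer and force feedback is present but disconnected, leaving Tick empty.
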(event `self.ReceiveTick`
  (params (DeltaSeconds :type "Float (single-precision)"))
  ;[1 0.187 0.177 1 50] Gamepad Shake
)

(event `Shake`
  ;[1 0.187 0.177 1 50] Gamepad Shake
  (`PlayerController.K2_ClientPlayForceFeedback` (`GameplayStatics.GetPlayerController` (`self.ID`)) "/Game/01_GD/FFB_Target.FFB_Target" "None" false false false)
  (`SceneComponent.SetVisibility` (`self.Drop`) true false))

(event `EnhancedInput|/Game/01_GD/Inputs/InputActions/IA_Move`
  (params (ActionValue :type "Vector2D Structure") (ElapsedSeconds :type "Float (double-precision)") (TriggeredSeconds :type "Float (double-precision)") (InputAction :type "InputAction Object Reference" :default "/Game/01_GD/Inputs/InputActions/IA_Move.IA_Move"))
  (bind _speed (`self.Speed`))
  ;[0.4842 0.6272 1 1 25] Movement
  (:`Triggered`
    (set `self.Axis2D` (`KismetMathLibrary.MakeVector2D` ActionValue_X ActionValue_Y))
    (`self.K2_AddActorLocalOffset` (`KismetMathLibrary.MakeVector` (* ActionValue_Y _speed) (* ActionValue_X _speed))))
  (:`Canceled`
    (set `self.Axis2D` (0.0 0.0) :!label _label))
  (:`Completed`
    (goto _label)))

(event `EnhancedInput|/Game/01_GD/Inputs/InputActions/IA_Attack`
  (params (ActionValue :type Boolean) (ElapsedSeconds :type "Float (double-precision)") (TriggeredSeconds :type "Float (double-precision)") (InputAction :type "InputAction Object Reference" :default "/Game/01_GD/Inputs/InputActions/IA_Attack.IA_Attack"))
  ;[1 0.3438 0.3438 1 25] Drop a Bom / Attack
  (:`Started`
    (if (`self.CanSpawn`)
      (set `self.CanSpawn` false)
      (`|SpawnActorFromClass` "/Game/01_GD/Gameplay/BP_Bomb.BP_Bomb_C" (`SceneComponent.K2_GetComponentToWorld` (`self.SpawnPoint`)) "Undefined" "MultiplyWithRoot" null null)
      (`KismetSystemLibrary.Delay` 1.5)
      (set `self.CanSpawn` true))))

(event `self.SuppPossessed`
  ;[0.5578 1 0.6824 1 25] On Possessed
  (`SceneComponent.SetVisibility` (`self.Decal`) true false)
  (`SceneComponent.SetVisibility` (`self.Drop`) true false)
  (set `self.CanShake?` true)
  (`KismetSystemLibrary.Delay` 3.0))

(fn `UserConstructionScript`
  (`parent.UserConstructionScript`))